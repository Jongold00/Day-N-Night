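; Base weapon Blueprint for BP_MainCharacter, handling hitscan firing, ammo and reloading for networked play.
; It takes its owner from the parent actor; firing checks ammo and holster state, then sends screen-center aim from the muzzle to a server RPC.
; That RPC line-traces, applies point damage and multicasts the fire montage.
; Reload multicasts its montage and refills ammo; both actions call dispatchers and briefly pulse state flags.
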(event Custom|RPC_StartShooting
  (params (Direction :type Vector) (Origin :type Vector) (Controller :type Player%20Controller%20Object%20Reference))
  ;[1 1 1] Server RPC to Fire Weapon
  (bind _outhit (Collision|LineTraceByChannel Origin (+ Origin (* Direction (Variables|Default|GetFireRange))) "TraceTypeQuery2" false (Utilities|Array|MakeArray (Variables|Default|GetAs%20BP%20Main%20Character)) "ForDuration"))
  (Variables|Default|SetOut%20Hit _outhit)
  (Utilities|FlowControl|Sequence
    (:then_0
      (CallFunction|MCFireBullet (Variables|Default|GetOut%20Hit) Direction)
      (Variables|Default|SetIsFire? true)
      (Utilities|FlowControl|Delay 0.01)
      (Variables|Default|SetIsFire? false))
    (:then_1
      (if (.bBlockingHit (Collision|BreakHitResult (Variables|Default|GetOut%20Hit)))
        (Game|Damage|ApplyPointDamage (.HitActor (Collision|BreakHitResult (Variables|Default|GetOut%20Hit))) (Variables|Default|GetBase%20Damage) (Math|Vector|GetUnitDirection(Vector) (.TraceStart (Collision|BreakHitResult (Variables|Default|GetOut%20Hit))) (.TraceEnd (Collision|BreakHitResult (Variables|Default|GetOut%20Hit)))) (Variables|Default|GetOut%20Hit) Controller self)))))

(event Custom|MC_FireBullet
  (params (HitResult :type Hit%20Result%20Structure) (Direction :type Vector))
  ;[1 1 1] Fire Weapon Animation Replicated Across all players
  (Animation|Montage|MontagePlay (Components|SkeletalMesh|GetAnimInstance (Variables|/Script/Engine.Character|GetMesh (Variables|Default|GetAs%20BP%20Main%20Character))) (Variables|Default|GetMontage%20to%20Play) 1.0 "MontageLength" 0.0 true))

(event Custom|MC_Reload
  ;[1 1 1] Reload Weapon
  (Animation|Montage|MontagePlay (Components|SkeletalMesh|GetAnimInstance (Variables|/Script/Engine.Character|GetMesh (Variables|Default|GetAs%20BP%20Main%20Character))) (Variables|Default|GetReloadMontage) 1.0 "MontageLength" 0.0 true)
  (Variables|Default|SetIsReloading? true)
  (Utilities|FlowControl|Delay 0.01)
  (Variables|Default|SetIsReloading? false))

(event EventPrimaryFire
  (params (IsFiring :type Boolean))
  (bind _returnvalue (Game|GetPlayerController 0))
  ;[1 1 1] Fire Event Interface
  (if IsFiring
    (if (and (> (Variables|Default|GetCurrentAmmo) 0) (not (Variables|/Game/Blueprints/Character/BP_MainCharacter.BP_MainCharacter_C|GetIsHolstered? (Variables|Default|GetAs%20BP%20Main%20Character))))
      (CallFunction|RPCStartShooting (.WorldDirection (Class|GameplayStatics|DeprojectScreentoWorld _returnvalue (- (/ (Viewport|GetViewportSize) (Math|Vector2D|MakeVector2D 2.0 2.0)) "(X=0.000000,Y=-10.000000)"))) (Transformation|GetWorldLocation (Variables|Default|GetMuzzle)) _returnvalue)
      (Variables|Default|SetCurrentAmmo (- (Variables|Default|GetCurrentAmmo) 1))
      (Default|CallOnShoot))))

(event EventBeginPlay
  ;[1 1 1] Init Owner of Weapon
  (bind _asbp_main_character (Utilities|Casting|CastToBP_MainCharacter (Actor|GetParentActor)))
  (bind _output_get (Variables|Default|SetAs%20BP%20Main%20Character _asbp_main_character))
  (Actor|SetOwner _output_get))

(event EventReload
  ;[1 1 1] Reload Weapon
  (CallFunction|MCReload)
  (Variables|Default|SetCurrentAmmo (Variables|Default|GetMaxAmmo))
  (Default|CallOnReloaded))

(fn ConstructionScript)