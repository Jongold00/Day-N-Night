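; Zombie enemy Blueprint that chases pawns it senses, takes point damage and dies at zero health.
; PawnSensing raises walk speed and drives AIMoveTo, while damage updates the overhead health bar through MC_UpdateHealthBar.
; Death, guarded by DoOnce, stops movement, clears the hasSeenPlayer blackboard key, flags IsDeath and destroys the actor after a delay.
; An authority-only CallOnDeath ragdoll function exists but is not called here, and setting hasSeenPlayer true is disconnected.
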(event OnSeePawn(PawnSensing)
  (params (Pawn :type Pawn%20Object%20Reference))
  (Variables|/Script/Engine.CharacterMovementComponent|SetMaxWalkSpeed (Variables|Character|GetCharacterMovement) 331.0)
  (AI|AIMoveTo self "0, 0, 0" Pawn 1e+02 false))

(event Custom|MC_UpdateHealthBar
  (bind _aswbp_overhead_health_bar (Utilities|Casting|CastToWBP_OverheadHealthBar (UserInterface|GetWidget (Variables|Default|GetOverheadWidget))))
  (Default|UpdateBar _aswbp_overhead_health_bar (Variables|Default|GetHealth) (Variables|Default|GetMaxHealth)))

(event Game|Damage|EventPointDamage
  (params (Damage :type Float%20%28single-precision%29) (DamageType :type Damage%20Type%20Object%20Reference) (HitLocation :type Vector :default "0, 0, 0") (HitNormal :type Vector :default "0, 0, 0") (HitComponent :type Primitive%20Component%20Object%20Reference) (BoneName :type Name :default "None") (ShotFromDirection :type Vector :default "0, 0, 0") (InstigatedBy :type Controller%20Object%20Reference) (DamageCauser :type Actor%20Object%20Reference) (HitInfo :type Hit%20Result%20Structure%20%28by%20ref%29))
  (Variables|Default|SetHealth (- (Variables|Default|GetHealth) Damage))
  (if (<= (Variables|Default|GetHealth) 0.0)
    (CallFunction|MCUpdateHealthBar)
    ;[1 1 1] Zombie Death
    (Utilities|FlowControl|DoOnce false
      (:Completed
        (Pawn|Components|CharacterMovement|DisableMovement (Variables|Character|GetCharacterMovement))
        (AI|Components|Blackboard|SetValueasBool (AI|GetBlackboard (AI|GetAIController self)) (Utilities|Name|MakeLiteralName "hasSeenPlayer") false)
        (Variables|Default|SetIsDeath? true)
        (Utilities|FlowControl|Delay 3.0)
        (Actor|DestroyActor)))
    (else
      (CallFunction|MCUpdateHealthBar))))

(fn ConstructionScript)

(fn CallonDeath
  (bind _mesh (Variables|Character|GetMesh))
  (Networking|SwitchHasAuthority
    (:Authority
      (Physics|SetSimulatePhysics _mesh true)
      (Physics|AddImpulse _mesh "1000.000000,1000.000000,1000.000000" "spine_01" true)
      (Collision|SetCollisionEnabled _mesh "QueryAndPhysics")
      (Collision|SetCollisionEnabled (Variables|Collision|GetCapsuleComponent) "NoCollision")
      (Variables|Default|SetHealth 0.0))))