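; Base pickup actor that lets an overlapping player character take a weapon.
; Entering the radius sets the owner, binds to the character's interact event and shows the pickup HUD for local players; leaving reverses this.
; Pickup forwards to SRV_Pickup, which asks the stored character to spawn the weapon on a socket and destroys the pickup on success.
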(event OnComponentBeginOverlap(PickupRadius)
  (params (OverlappedComponent :type Primitive%20Component%20Object%20Reference) (OtherActor :type Actor%20Object%20Reference) (OtherComp :type Primitive%20Component%20Object%20Reference) (OtherBodyIndex :type Integer) (bFromSweep :type Boolean) (SweepResult :type Hit%20Result%20Structure%20%28by%20ref%29))
  ;[1 1 1] Overlapping Events
  (bind _asbp_player_character (Utilities|Casting|CastToBP_Player_Character OtherActor))
  (bind _output_get (Variables|Default|SetAs%20BP%20Player%20Character _asbp_player_character))
  (Actor|SetOwner _output_get)
  (EventDispatchers|BindEventtoInteract _asbp_player_character (EventDispatchers|CreateEvent :!event Custom|Pickup))
  (if (Pawn|IsLocallyControlled _asbp_player_character)
    (if (not (UserInterface|Viewport|IsinViewport (Variables|/Game/Blueprints/Character/BP_Player_Character.BP_Player_Character_C|GetPickupUI%20HUD%20Ref _asbp_player_character)))
      (UserInterface|Viewport|AddtoViewport (Variables|/Game/Blueprints/Character/BP_Player_Character.BP_Player_Character_C|GetPickupUI%20HUD%20Ref _asbp_player_character) 0))))

(event OnComponentEndOverlap(PickupRadius)
  (params (OverlappedComponent :type Primitive%20Component%20Object%20Reference) (OtherActor :type Actor%20Object%20Reference) (OtherComp :type Primitive%20Component%20Object%20Reference) (OtherBodyIndex :type Integer))
  ;[1 1 1] Overlapping Events
  (bind _asbp_player_character (Utilities|Casting|CastToBP_Player_Character OtherActor))
  (Variables|Default|SetAs%20BP%20Player%20Character _asbp_player_character)
  (Actor|SetOwner 0)
  (EventDispatchers|UnbindEventfromInteract _asbp_player_character (EventDispatchers|CreateEvent :!event Custom|Pickup))
  (if (Pawn|IsLocallyControlled _asbp_player_character)
    (Widget|RemovefromParent (Variables|/Game/Blueprints/Character/BP_Player_Character.BP_Player_Character_C|GetPickupUI%20HUD%20Ref _asbp_player_character))))

(event Custom|Pickup
  ;[1 1 1] Pickup Event
  (CallFunction|SRVPickup))

(event Custom|SRV_Pickup
  ;[1 1 1] Pickup Event
  (bind _as_bp_player_character (Variables|Default|GetAs%20BP%20Player%20Character)
    (:then
      (bind _success (Default|SpawnWeapon _as_bp_player_character (Variables|Default|GetObject) (Variables|Default|GetWeaponSocket)))
      (if _success
        (Actor|DestroyActor)))
    (:else)))

(fn ConstructionScript)